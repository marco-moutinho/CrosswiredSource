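; BP_CwPlayerChar is the player character, routing Enhanced Input to movement, look, jump, interaction and weapon use.
; On BeginPlay it passes its capsule radius to the MJS movement component.
; Primary action traces through WeaponUser, shows blocking hits as crosshair obstructions on the controller's HUD, then fires the current weapon.
; A hardcoded Q key equips holster slot 0 at Arrow1; older async weapon-spawning logic remains disconnected.
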(event `self.ReceiveBeginPlay`
  (`JumpStartMovementComponent.Function_SetCapsuleRadiusRefValue` (`self.M_JSMovementCompPtr`) (`CapsuleComponent.CapsuleRadius` (`self.CapsuleComponent`))))

(event `EnhancedInput|/CCC_JumpStart_Plugin/Input/IA_Move`
  (params (ActionValue :type "Vector2D Structure") (ElapsedSeconds :type "Float (double-precision)") (TriggeredSeconds :type "Float (double-precision)") (InputAction :type "InputAction Object Reference" :default "/CCC_JumpStart_Plugin/Input/IA_Move.IA_Move"))
  (:`Triggered`
    (`self.Function_MoveSimple` ActionValue :!label _label))
  (:`Started`
    (goto _label))
  (:`Canceled`
    (goto _label))
  (:`Completed`
    (goto _label)))

(event `EnhancedInput|/CCC_JumpStart_Plugin/Input/IA_Look`
  (params (ActionValue :type "Vector2D Structure") (ElapsedSeconds :type "Float (double-precision)") (TriggeredSeconds :type "Float (double-precision)") (InputAction :type "InputAction Object Reference" :default "/CCC_JumpStart_Plugin/Input/IA_Look.IA_Look"))
  (:`Triggered`
    (`self.Function_LookSimple` ActionValue 1.0 true)))

(event `EnhancedInput|/CCC_JumpStart_Plugin/Input/IA_Interact`
  (params (ActionValue :type Boolean) (ElapsedSeconds :type "Float (double-precision)") (TriggeredSeconds :type "Float (double-precision)") (InputAction :type "InputAction Object Reference" :default "/CCC_JumpStart_Plugin/Input/IA_Interact.IA_Interact"))
  (:`Started`
    (`self.Function_TraceFromPOV`)))

(event `EnhancedInput|/CCC_JumpStart_Plugin/Input/IA_Jump`
  (params (ActionValue :type Boolean) (ElapsedSeconds :type "Float (double-precision)") (TriggeredSeconds :type "Float (double-precision)") (InputAction :type "InputAction Object Reference" :default "/CCC_JumpStart_Plugin/Input/IA_Jump.IA_Jump"))
  (:`Started`
    (`self.Jump`))
  (:`Canceled`
    (`self.StopJumping` :!label _label_2))
  (:`Completed`
    (goto _label_2)))

(event `EnhancedInput|/CCC_JumpStart_Plugin/Input/IA_PrimaryAction`
  (params (ActionValue :type Boolean) (ElapsedSeconds :type "Float (double-precision)") (TriggeredSeconds :type "Float (double-precision)") (InputAction :type "InputAction Object Reference" :default "/CCC_JumpStart_Plugin/Input/IA_PrimaryAction.IA_PrimaryAction"))
  (bind (_asbp_cw_player_controller _bsuccess) (cast `/Game/GameBasics/BP_CwPlayerController` (`GameplayStatics.GetPlayerController` 0) :!pure true))
  (:`Started`
    (`|ExecutionSequence`
      (:`then_0`
        (bind _outhitresult (`WeaponUser.Function_TraceFromPov` (`self.WeaponUser`)))
        (bind (_bblockinghit _binitialoverlap _time _distance _location _impactpoint) (`GameplayStatics.BreakHitResult` _outhitresult))
        (if _bblockinghit
          (if _bsuccess
            (`WD_HUD.Function_UpdateCrosshairObstructionPosition` (`JumpStartController.M_MainHudPtr` _asbp_cw_player_controller) _impactpoint true)
            (else
              (`KismetSystemLibrary.PrintString` "FALSe")))))
      (:`then_1`
        (`WeaponUser.Function_UseCurrentWeapon` (`self.WeaponUser`) "IP_OnStartPress")))))

(event `Key|Q`
  (params (Key :type "Key Structure"))
  (bind _weaponuser (`self.WeaponUser`))
  (:`Pressed`
    (set `WeaponUser.PH_WeaponAttachPoint` (`self.Arrow1`) _weaponuser)
    (`WeaponUser.Function_EquipWeaponAdvanced` _weaponuser 0 null)))

(fn `UserConstructionScript`
  (`parent.UserConstructionScript`))