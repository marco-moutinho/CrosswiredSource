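; Player controller that sets up Enhanced Input and gives the player a Tab-toggled map changer widget.
; BeginPlay calls the input subsystem initializer, then creates BP_MapChanger and adds it to the viewport hidden.
; Tab flips the widget's visibility, switching the mouse cursor and input mode between game-only and game-and-UI with the widget focused.
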(event `self.ReceiveBeginPlay`
  (`self.Method_InitializeEnhancedInputSubsystem`)
  (bind _returnvalue (`|CreateWidget` "/Game/Widgets/BP_MapChanger.BP_MapChanger_C" self))
  (bind _output_get (set `self.WdMapChanger` _returnvalue))
  (`UserWidget.AddToViewport` _output_get 1)
  (`Widget.SetVisibility` _output_get "Hidden"))

(event `Key|Tab`
  (params (Key :type "Key Structure"))
  (bind _wdmapchanger (`self.WdMapChanger`))
  (:`Pressed`
    (switch `ESlateVisibility` (`Widget.GetVisibility` _wdmapchanger)
      (:`Visible`
        (`Widget.SetVisibility` _wdmapchanger "Hidden")
        (set `self.bShowMouseCursor` false)
        (`WidgetBlueprintLibrary.SetInputMode_GameOnly` self))
      (:`Hidden`
        (`Widget.SetVisibility` _wdmapchanger "Visible")
        (set `self.bShowMouseCursor` true)
        (`WidgetBlueprintLibrary.SetInputMode_GameAndUIEx` self _wdmapchanger)))))

(fn `UserConstructionScript`)